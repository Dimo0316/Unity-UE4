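; Dynamic foliage actor that physically reacts to nearby "FO"-tagged actors, standing in for a foliage instance.
; A radius sphere tracks those actors, and each tick the nearest one's distance drives an interpolated physics blend weight on the skeletal mesh.
; When none remain in range, it re-adds an instance to the source foliage component, deregisters from the game state and destroys itself.
; A separate DoSmooth event can fade the blend through a timeline.
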(event OnComponentBeginOverlap(Sphere)
  (params (OverlappedComponent :type Primitive%20Component%20Object%20Reference) (OtherActor :type Actor%20Object%20Reference) (OtherComp :type Primitive%20Component%20Object%20Reference) (OtherBodyIndex :type Integer) (bFromSweep :type Boolean) (SweepResult :type Hit%20Result%20Structure%20%28by%20ref%29))
  (CallFunction|RegistInteractiveActor OtherActor))

(event OnComponentEndOverlap(Sphere)
  (params (OverlappedComponent :type Primitive%20Component%20Object%20Reference) (OtherActor :type Actor%20Object%20Reference) (OtherComp :type Primitive%20Component%20Object%20Reference) (OtherBodyIndex :type Integer))
  (CallFunction|UnRegistInteractiveActor OtherActor))

(event Custom|DoSmooth
  (params (fadein :type Boolean))
  (Components|Timeline|SetPlayRate (Variables|Default|GetSmoothPhy) 0.5)
  (if fadein
    (bind _alpha (Timeline|SmoothPhy PlayFromStart)
      (:Update
        (Class|SkeletalMeshComponent|SetAllBodiesBelowPhysicsBlendWeight (Variables|Default|GetSkeletalMesh) (Variables|Default|Getbone) _alpha false true)))
    (else
      (Timeline|SmoothPhy ReverseFromEnd))))

(event EventBeginPlay)

(event EventTick
  (params (DeltaSeconds :type Float%20%28single-precision%29))
  (CallFunction|UpdatePhyWeight))

(fn ConstructionScript
  (Components|Sphere|SetSphereRadius (Variables|Default|GetSphere) (Variables|Default|GetPhyRadius) true))

(fn UpdatePhyWeight
  (bind _interactiveactors (Variables|Default|GetInteractiveActors))
  (bind _phyradius (Variables|Default|GetPhyRadius))
  (bind _returnvalue (* _phyradius 0.8))
  ;[1 0 0] should KEEP enough buffer
  (bind _output_get (LocalVariables|SetlocThreshold (+ (Variables|Default|GetPhyRadius) 1.5e+02)))
  (Variables|Default|SetcurDist _output_get)
  (Utilities|FlowControl|Sequence
    (:then_0
      (for (_array_element _array_index) _interactiveactors
        (Utilities|IsValid _array_element
          (:Is%20Valid
            (if (< (Transformation|GetDistanceTo _array_element self) (Variables|Default|GetcurDist))
              (Variables|Default|SetcurDist (Transformation|GetDistanceTo _array_element self))))
          (:Is%20Not%20Valid
            (Utilities|Array|RemoveIndex _interactiveactors _array_index)))))
    (:then_1
      (if (== (Utilities|Array|Length _interactiveactors) 0)
        (CallFunction|DoDestroy :!label _label)
        (else
          (bind _output_get_2 (Variables|Default|SetcurWeight (Math|Interpolation|FInterpTo (Variables|Default|GetcurWeight) (Math|Float|MapRangeClamped (Variables|Default|GetcurDist) (Math|Float|Clamp(Float) _returnvalue 3.5e+02 _returnvalue) 1.5e+02 0.0 1.0) (Utilities|Time|GetWorldDeltaSeconds) 8.0)))
          (if (>= (Variables|Default|GetcurDist) (LocalVariables|GetlocThreshold))
            (goto _label)
            (else
              (Class|SkeletalMeshComponent|SetAllBodiesBelowPhysicsBlendWeight (Variables|Default|GetSkeletalMesh) (Variables|Default|Getbone) _output_get_2 false true))))))))

(fn RegistInteractiveActor
  (params (actor :type Actor%20Object%20Reference))
  (if (Actor|ActorHasTag actor "FO")
    (Utilities|Array|AddUnique (Variables|Default|GetInteractiveActors) actor)))

(fn UnRegistInteractiveActor
  (params (actor :type Actor%20Object%20Reference))
  (Utilities|Array|RemoveItem (Variables|Default|GetInteractiveActors) actor))

(fn DoDestroy
  (bind _foliageactor (Variables|Default|GetFoliageActor))
  (Utilities|FlowControl|Sequence
    (:then_0
      (Utilities|IsValid _foliageactor
        (:Is%20Valid
          (Class|InstancedStaticMeshComponent|AddInstanceWorldSpace (Utilities|Array|Get(acopy) (Actor|GetComponentsByClass _foliageactor "/Game/Assets/PhyFoliageInstancedSMComponent.PhyFoliageInstancedSMComponent_C") (Variables|Default|GetcomIndex)) (Transformation|GetActorTransform)))))
    (:then_1
      (bind _asmy_game_state (Utilities|Casting|CastToMyGameState (Game|GetGameState)))
      (Default|RemoveDynFoliage _asmy_game_state self))
    (:then_2
      (Actor|DestroyActor))))